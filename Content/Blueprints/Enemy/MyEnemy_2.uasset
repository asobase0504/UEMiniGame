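; MyEnemy_2 is an enemy Blueprint that adjusts Player 1's score when it is destroyed after being hit.
; On Destroyed, it checks IsHit, then casts the game mode to BP_MyGameModeBase and adds its Score to Player1Score.
; The total is floored at zero, so a negative Score cannot push the player's score below zero.
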(event `self.ReceiveDestroyed`
  (if (`self.IsHit`)
    (bind _asbp_my_game_mode_base (cast `/Game/UI/BP/BP_MyGameModeBase` (`GameplayStatics.GetGameMode`)))
    (bind _returnvalue (+ (`/Game/UI/BP/BP_MyGameModeBase.Player1Score` _asbp_my_game_mode_base) (`self.Score`)))
    (if (< _returnvalue 0)
      (set `/Game/UI/BP/BP_MyGameModeBase.Player1Score` 0 _asbp_my_game_mode_base)
      (else
        (set `/Game/UI/BP/BP_MyGameModeBase.Player1Score` _returnvalue _asbp_my_game_mode_base)))))

(fn `UserConstructionScript`)